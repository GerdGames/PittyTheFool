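; BP_Roller is an interactable actor that rolls to a preset end transform in response to a Joke event.
; A timeline lerps the actor from its current transform to RollEndTransform, then runs a fall check.
; The check line-traces downward to compute FallEndTransform above the hit point and starts a second timeline.
; That second timeline still lerps toward RollEndTransform, leaving the computed fall target unused.
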(event `/Game/PittyTheFool/Code/Interactables/Interfaces/Int_Joke_Able.ReceiveJoke`
  (params (JokeType :type "/Game/PittyTheFool/Code/Jokes/Enum_Joke Enum" :default "NewEnumerator0"))
  (switch `/Game/PittyTheFool/Code/Jokes/Enum_Joke` JokeType
    (:`NewEnumerator0`
      (`self.Roll`))))

(event `Roll`
  ;[1 1 1] Roll
  (set `self.StartTransform` (`self.GetTransform`))
  (bind (_direction _newtrack_0) (`Timeline|Timeline`)
    (:`Update`
      (`self.K2_SetActorTransform` (`KismetMathLibrary.TLerp` (`self.StartTransform`) (`self.RollEndTransform`) _newtrack_0)))
    (:`Finished`
      (`self.Check to Fall`))))

(event `Check to Fall`
  (bind _returnvalue (`self.K2_GetActorLocation`))
  ;[1 1 1] Check to Fall
  (bind _outhit (`KismetSystemLibrary.LineTraceSingleByProfile` :`Start` (+ _returnvalue (0.0 0.0 -50.0)) :`End` (+ _returnvalue (0.0 0.0 -10000.0)) :`ProfileName` "BlockAll" :`DrawDebugType` "ForDuration"))
  (set `self.FallEndTransform` (`KismetMathLibrary.MakeTransform` (+ (`.Location` (`GameplayStatics.BreakHitResult` _outhit)) (0.0 0.0 50.0))))
  (set `self.StartTransform` (`self.GetTransform`))
  (bind (_direction _newtrack_0) (`Timeline|Timeline_0` :!via `PlayFromStart`)
    (:`Update`
      (`self.K2_SetActorTransform` (`KismetMathLibrary.TLerp` (`self.StartTransform`) (`self.RollEndTransform`) _newtrack_0)))))

(fn `UserConstructionScript`)