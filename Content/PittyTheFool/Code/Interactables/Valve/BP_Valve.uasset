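; Valve interactable that toggles a referenced water actor between high and low levels when it receives a Rolling joke.
; The Joke event calls Flow behind a DoOnce, which resets after a three-second delay for that joke type only.
; Flow flips the level state and uses a Timeline to lerp the water by a positive or negated offset.
; Water is unhidden before rising and hidden after lowering finishes.
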(event `self.ReceiveBeginPlay`
  (set `self.Low Water Level Offset` (`self.K2_GetActorLocation` (`self.WaterReference`))))

(event `self.ReceiveJoke`
  (params (JokeType :type "/Game/PittyTheFool/Code/Jokes/Enum_Joke Enum" :default "NewEnumerator0"))
  (`/Engine/EditorBlueprintResources/StandardMacros.DoOnce` false :!label _label
    (:`Completed`
      (switch `/Game/PittyTheFool/Code/Jokes/Enum_Joke` JokeType
        (:`NewEnumerator0`
          (`self.Flow`)
          (`KismetSystemLibrary.Delay` 3.0)
          (goto _label :!via `Reset`))))))

(event `Flow`
  (bind _waterstartposition (`self.WaterStartPosition`))
  ;[1 1 1] Flow
  (`|ExecutionSequence`
    (:`then_0`
      (if (`self.WaterLevelHigh`)
        (set `self.WaterLevelHigh` false)
        (set `self.WaterLevelOffset` (* (`self.HighWaterLevelOffset`) -1.0))
        (else
          (set `self.WaterLevelHigh` true)
          (`self.SetActorHiddenInGame` (`self.WaterReference`) false)
          (set `self.WaterLevelOffset` (`self.HighWaterLevelOffset`)))))
    (:`then_2`
      (set `self.WaterStartPosition` (`self.K2_GetActorLocation` (`self.WaterReference`)))
      (bind (_direction _newtrack_0) (`Timeline|Timeline`)
        (:`Update`
          (`self.K2_SetActorLocation` (`self.WaterReference`) (`KismetMathLibrary.VLerp` _waterstartposition (+ _waterstartposition (`self.WaterLevelOffset`)) _newtrack_0) false false))
        (:`Finished`
          (if (not (`self.WaterLevelHigh`))
            (`self.SetActorHiddenInGame` (`self.WaterReference`) true)))))))

(fn `UserConstructionScript`)