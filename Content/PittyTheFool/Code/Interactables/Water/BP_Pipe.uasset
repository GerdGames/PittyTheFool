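; BP_Pipe is an interactable pipe that starts flowing when it receives a Crack Up joke.
; Flow runs only while the Panel component is valid, destroying it and unhiding the referenced water actor.
; A timeline then lerps the water from its current location by WaterLevelOffset to shift the water level.
; Two audio components are added, the second after a short delay.
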(event `self.ReceiveJoke`
  (params (JokeType :type "/Game/PittyTheFool/Code/Jokes/Enum_Joke Enum" :default "NewEnumerator0"))
  (switch `/Game/PittyTheFool/Code/Jokes/Enum_Joke` JokeType
    (:`NewEnumerator2`
      (`self.Flow`))))

(event `Flow`
  (bind _waterstartposition (`self.WaterStartPosition`))
  ;[1 1 1] Start Flowing
  (if (`KismetSystemLibrary.IsValid` (`self.Panel`))
    (`|ExecutionSequence`
      (:`then_0`
        (`ActorComponent.K2_DestroyComponent` (`self.Panel`)))
      (:`then_1`
        (`self.SetActorHiddenInGame` (`self.WaterReference`) false))
      (:`then_2`
        (set `self.WaterStartPosition` (`self.K2_GetActorLocation` (`self.WaterReference`)))
        (bind (_direction _newtrack_0) (`Timeline|Timeline` :!via `PlayFromStart`)
          (:`Update`
            (`self.K2_SetActorLocation` (`self.WaterReference`) (`KismetMathLibrary.VLerp` _waterstartposition (+ _waterstartposition (`self.WaterLevelOffset`)) _newtrack_0) false false))))
      (:`then_3`
        (`AddComponent|NODE_AddAudioComponent-1`))
      (:`then_4`
        (`KismetSystemLibrary.Delay` 0.2)
        (`AddComponent|NODE_AddAudioComponent-0`)))))

(fn `UserConstructionScript`)