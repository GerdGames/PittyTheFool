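; BP_Gem_Collectable is a gem pickup that comes in Stoat, Goat and Axolotl types.
; The construction script sets the gem's material from its GemType.
; On BeginPlay it caches the Fool_GameInstance.
; On overlap with any actor, it marks its type as collected in the instance's GemsCollected map, then destroys itself.
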(event `self.ReceiveBeginPlay`
  (bind _asfool_game_instance (cast `/Game/PittyTheFool/Code/GameMode/Fool_GameInstance` (`GameplayStatics.GetGameInstance`)))
  (set `self.FoolGameInst` _asfool_game_instance))

(event `self.ReceiveActorBeginOverlap`
  (params (OtherActor :type "Actor Object Reference"))
  (`|ExecutionSequence`
    (:`then_0`
      (`BlueprintMapLibrary.Map_Add` (`/Game/PittyTheFool/Code/GameMode/Fool_GameInstance.GemsCollected` (`self.FoolGameInst`)) (`self.GemType`) true))
    (:`then_1`
      (`self.K2_DestroyActor`))))

(fn `UserConstructionScript`
  (`PrimitiveComponent.SetMaterial` (`self.Gem`) 0 (select `/Game/PittyTheFool/Code/Interactables/Gem/GemType` (`self.GemType`) :`NewEnumerator0` "/Game/PittyTheFool/Art/TrevorModels/Gem/MI_Stoat_Gem.MI_Stoat_Gem" :`NewEnumerator1` "/Game/PittyTheFool/Art/TrevorModels/Gem/MI_Goat_Gem.MI_Goat_Gem" :`NewEnumerator2` "/Game/PittyTheFool/Art/TrevorModels/Gem/MI_Axolotl_Gem.MI_Axolotl_Gem" :!type "MaterialInterface Object Reference")))