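; BP_Plant is an interactable plant that grows in response to a Crying joke.
; Its Joke event switches on the joke type and calls Grow only for Crying.
; Grow captures the current transform, then a timeline lerps the actor toward a location shifted by EndTransformOffset, keeping rotation and using the offset's scale as the final scale.
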(event `self.ReceiveJoke`
  (params (JokeType :type "/Game/PittyTheFool/Code/Jokes/Enum_Joke Enum" :default "NewEnumerator0"))
  (switch `/Game/PittyTheFool/Code/Jokes/Enum_Joke` JokeType
    (:`NewEnumerator1`
      (`self.Grow`))))

(event `Grow`
  (bind _starttransform (`self.StartTransform`))
  ;[1 1 1] Roll
  (set `self.StartTransform` (`self.GetTransform`))
  (bind (_direction _newtrack_0) (`Timeline|Timeline`)
    (:`Update`
      (`self.K2_SetActorTransform` (`KismetMathLibrary.TLerp` _starttransform (`KismetMathLibrary.MakeTransform` (+ (.location _starttransform) (.location (`self.EndTransformOffset`))) (.rotation _starttransform) (.scale (`self.EndTransformOffset`))) _newtrack_0)))))

(fn `UserConstructionScript`)