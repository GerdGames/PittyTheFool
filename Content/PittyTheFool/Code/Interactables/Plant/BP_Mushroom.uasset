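; BP_Mushroom is an interactable plant that reacts to jokes and bounces the player character, BP_TheFool, on contact.
; A Crying joke triggers growth and a success sound, while Rolling and Crack Up only play a fail sound.
; Growth uses a timeline to lerp position and scale toward EndTransformOffset, then sets the launch force.
; Hits apply that force to the Fool as a velocity-change impulse against the hit normal.
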(event `self.ReceiveJoke`
  (params (JokeType :type "/Game/PittyTheFool/Code/Jokes/Enum_Joke Enum" :default "NewEnumerator0"))
  (switch `/Game/PittyTheFool/Code/Jokes/Enum_Joke` JokeType
    (:`NewEnumerator0`
      (`KismetSystemLibrary.Delay` 0.5 :!label _label)
      (`GameplayStatics.PlaySound2D` "/Game/Audio/Crowd-20240805T004618Z-001/Crowd/Fail_Cue.Fail_Cue" 1.0 1.0 0.0 null null))
    (:`NewEnumerator1`
      (`self.Grow`)
      (`KismetSystemLibrary.Delay` 0.5)
      (`GameplayStatics.PlaySound2D` "/Game/Audio/Crowd-20240805T004618Z-001/Crowd/Success_Cue.Success_Cue" 1.0 1.0 0.0 null null))
    (:`NewEnumerator2`
      (goto _label))))

(event `Grow`
  (bind _returnvalue (`self.GetTransform`))
  (bind _starttransform (`self.StartTransform`))
  ;[1 1 1] Grow
  (set `self.StartTransform` _returnvalue)
  (`GameplayStatics.PlaySoundAtLocation` "/Game/Audio/Mushroom_Growth.Mushroom_Growth" (.location _returnvalue) (struct) 1.0 1.0 0.0 null null null null)
  (bind (_direction _newtrack_0) (`Timeline|Timeline`)
    (:`Update`
      (`self.K2_SetActorTransform` (`KismetMathLibrary.TLerp` _starttransform (`KismetMathLibrary.MakeTransform` (+ (.location _starttransform) (.location (`self.EndTransformOffset`))) (.rotation _starttransform) (.scale (`self.EndTransformOffset`))) _newtrack_0)))
    (:`Finished`
      (set `self.LaunchForce` 1000.0))))

(event `self.ReceiveHit`
  (params (MyComp :type "PrimitiveComponent Object Reference") (Other :type "Actor Object Reference") (OtherComp :type "PrimitiveComponent Object Reference") (bSelfMoved :type Boolean) (HitLocation :type "Vector Structure") (HitNormal :type "Vector Structure") (NormalImpulse :type "Vector Structure") (Hit :type "HitResult Structure (by ref)"))
  (bind _asbp_the_fool (cast `/Game/PittyTheFool/Code/TheFool/BP_TheFool` Other))
  (`CharacterMovementComponent.AddImpulse` (`Character.CharacterMovement` _asbp_the_fool) (* (* HitNormal -1.0) (`self.LaunchForce`)) true)
  (`GameplayStatics.PlaySoundAtLocation` "/Game/Audio/Mushroom_Bounce_Cue.Mushroom_Bounce_Cue" HitLocation (struct) 1.0 1.0 0.0 null null null null))

(fn `UserConstructionScript`)